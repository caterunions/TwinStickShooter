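; Player hero character for a cursor-aimed shooter with an orthographic camera, mouse-wheel zoom and camera-relative movement.
; Each tick it turns the controller toward the point under the cursor and snaps mesh yaw to 45-degree steps; look axes can also set control rotation.
; BeginPlay spawns and attaches BP_Weapon at GunTemp, and the left mouse button starts and stops firing.
; AffectHealth recalculates health and destroys the actor on death.
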(event EventBeginPlay
  ;[0.15 0.15 0.15 0.5] BeginPlay
  (Utilities|FlowControl|Sequence
    (:then_0
      ;[0.15 0.15 0.15 0.5] Spawn Weapon
      (bind _returnvalue (Game|SpawnActorfromClass "/Game/Blueprints/BP_Weapon.BP_Weapon_C" (Transformation|GetWorldTransform (Variables|Default|Getgun%20temp)) "Undefined" "MultiplyWithRoot" 0 0))
      (bind _output_get (Variables|Default|SetWeapon _returnvalue))
      (Transformation|AttachComponentToComponent _output_get (Variables|Default|Getgun%20temp) "None" "SnapToTarget" "SnapToTarget" "KeepWorld" true))))

(event EventAffectHealth
  (params (Delta :type Float%20%28double-precision%29))
  ;[0.15 0.15 0.15 0.5] Damage Calculation
  (CallFunction|CalculateHealth Delta)
  (if (CallFunction|IsDead)
    (Actor|DestroyActor)))

(event EventTick
  (params (DeltaSeconds :type Float%20%28single-precision%29))
  (bind _returnvalue (Game|GetPlayerController 0))
  (bind _returnvalue_2 (Transformation|GetActorLocation))
  (bind _hitresult (Game|Player|GetHitResultUnderCursorbyChannel _returnvalue "TraceTypeQuery1" true))
  (bind _returnvalue_3 (Math|Rotator|FindLookatRotation _returnvalue_2 (.location _hitresult)))
  ;[0.15 0.15 0.15 0.5] Mouse rotation!
  (Pawn|SetControlRotation (Pawn|GetController) _returnvalue_3)
  (CallFunction|QuantizeMeshRotation _returnvalue_3))

(event Input|AxisEvents|InputAxisMoveUp
  (params (AxisValue :type Float%20%28single-precision%29))
  (bind _camera (Variables|Default|GetCamera))
  (bind _returnvalue (Math|Vector|GetForwardVector _camera))
  ;[0.15 0.15 0.15 0.5] Movement
  (Pawn|Input|AddMovementInput (Math|Vector|Normalize (Math|Vector|MakeVector (.x _returnvalue) (.y _returnvalue) 0.0)) AxisValue false))

(event Input|AxisEvents|InputAxisMoveRight
  (params (AxisValue :type Float%20%28single-precision%29))
  ;[0.15 0.15 0.15 0.5] Movement
  (Pawn|Input|AddMovementInput (Math|Vector|GetRightVector (Variables|Default|GetCamera)) AxisValue false))

(event Input|AxisEvents|InputAxisLookRight
  (params (AxisValue :type Float%20%28single-precision%29))
  ;[0.15 0.15 0.15 0.5] Controller/Arrow Key Rotation
  (if (> (Math|Vector|VectorLength (Math|Vector|MakeVector (stale Input|AxisEvents|InputAxisLookUp AxisValue) AxisValue 0.0)) 0.25)
    (Pawn|SetControlRotation (Pawn|GetController) (Math|Conversions|RotationFromXVector (Math|Vector|MakeVector (stale Input|AxisEvents|InputAxisLookUp AxisValue) AxisValue 0.0)))))

(event Input|AxisEvents|InputAxisLookUp
  (params (AxisValue :type Float%20%28single-precision%29))
  ;[0.15 0.15 0.15 0.5] Controller/Arrow Key Rotation
  (if (> (Math|Vector|VectorLength (Math|Vector|MakeVector AxisValue (stale Input|AxisEvents|InputAxisLookRight AxisValue) 0.0)) 0.25)
    (Pawn|SetControlRotation (Pawn|GetController) (Math|Conversions|RotationFromXVector (Math|Vector|MakeVector AxisValue (stale Input|AxisEvents|InputAxisLookRight AxisValue) 0.0)))))

(event Input|MouseEvents|MouseWheelDown
  (params (Key :type Key%20Structure :default "None"))
  (bind _camera (Variables|Default|GetCamera))
  (bind _orthowidth (Variables|/Script/Engine.CameraComponent|GetOrthoWidth _camera))
  ;[0.15 0.15 0.15 0.5] Scroll to adjust camera zoom
  (:Pressed
    (Class|CameraComponent|SetOrthoWidth _camera (Math|Float|Min(Float) (+ _orthowidth (/ _orthowidth 1e+01)) 5e+03))))

(event Input|MouseEvents|MouseWheelUp
  (params (Key :type Key%20Structure :default "None"))
  (bind _camera (Variables|Default|GetCamera))
  (bind _orthowidth (Variables|/Script/Engine.CameraComponent|GetOrthoWidth _camera))
  ;[0.15 0.15 0.15 0.5] Scroll to adjust camera zoom
  (:Pressed
    (Class|CameraComponent|SetOrthoWidth _camera (Math|Float|Max(Float) (- _orthowidth (/ _orthowidth 1e+01)) 1e+03))))

(event Input|MouseEvents|LeftMouseButton
  (params (Key :type Key%20Structure :default "None"))
  (bind _weapon (Variables|Default|GetWeapon))
  ;[0.15 0.15 0.15 0.5] Fire Weapon
  (:Pressed
    (Default|BeginFiring _weapon))
  (:Released
    (Default|EndFiring _weapon)))

(fn ConstructionScript
  (|CallParentFunction))

(fn QuantizeMeshRotation
  (params (RealRotation :type Rotator))
  (Transformation|SetWorldRotation (Variables|Character|GetMesh) (Math|Rotator|MakeRotator 0.0 0.0 (Math|Conversions|ToFloat(Integer) (- (* (Math|Float|Round (/ (.yaw RealRotation) 45.0)) 45) 90))) false false))