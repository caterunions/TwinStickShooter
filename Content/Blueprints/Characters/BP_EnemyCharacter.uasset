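; Enemy character for a twin-stick game that damages the hero in melee and awards score when killed.
; AffectHealth (IDamageable) updates health and spawns a damage number; death adds score via BP_TwinStickMode, detaches the controller, drops some collision, then destroys the actor.
; BeginAttack opens a timed, DoOnce-gated attack state, while EnableAttackHitbox separately damages a hero overlapping DamageVolume.
; Tick snaps mesh yaw to eight directions; construction tints the body material.
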(event Custom|DamageHero
  ;[0.15 0.15 0.15 0.5] DamageHero
  (Default|AffectHealth (Variables|Default|GetHero) (* (Variables|Default|GetDamage) -1.0)))

(event Custom|EnableAttackHitbox
  ;[0.15 0.15 0.15 0.5] Attack
  (if (not (CallFunction|IsDead))
    (bind _asbp_hero_character (Utilities|Casting|CastToBP_HeroCharacter (Utilities|Array|Get(acopy) (Collision|GetOverlappingActors (Variables|Default|GetDamageVolume) "/Game/Blueprints/Characters/BP_HeroCharacter.BP_HeroCharacter_C" :!class /Script/Engine.PrimitiveComponent))))
    (Variables|Default|SetHero _asbp_hero_character)
    (CallFunction|DamageHero)))

(event Custom|BeginAttack
  (Utilities|FlowControl|DoOnce false
    (:Completed
      (Variables|Default|SetAttacking true)
      (Utilities|Time|SetTimerbyEvent (delegate Custom|EndAttack) (Variables|Default|GetAttackDuration)))))

(event Custom|EndAttack
  (Variables|Default|SetAttacking false)
  (Utilities|FlowControl|DoOnce false) ; enters at Reset
)

(event EventTick
  (params (DeltaSeconds :type Float%20%28single-precision%29))
  ;[0.15 0.15 0.15 0.5] Event Tick
  (CallFunction|QuantizeMeshRotation (Transformation|GetWorldRotation (Variables|Default|GetCapsuleComponent))))

(event EventAffectHealth
  (params (Delta :type Float%20%28double-precision%29))
  (bind _returnvalue (Transformation|GetActorLocation))
  ;[0.15 0.15 0.15 0.5] Implement IDamageable
  (CallFunction|CalculateHealth Delta)
  (Game|SpawnActorfromClass "/Game/Blueprints/BP_DamageNumber.BP_DamageNumber_C" (Math|Transform|MakeTransform (Math|Vector|MakeVector (.x _returnvalue) (.y _returnvalue) (+ (.z _returnvalue) (.z (.BoxExtent (Collision|GetComponentBounds (Variables|Default|GetCapsuleComponent)))))) "45.000000,145.000000,0.000000" "1.000000,1.000000,1.000000") "AlwaysSpawn" "MultiplyWithRoot" 0 Delta 0)
  (if (CallFunction|IsDead)
    (bind _asbp_twin_stick_mode (Utilities|Casting|CastToBP_TwinStickMode (Game|GetGameMode)))
    (Default|IncrementScore _asbp_twin_stick_mode (Variables|Default|GetScoreValue))
    (Class|Pawn|DetachfromControllerPendingDestroy)
    (Collision|SetCollisionResponsetoChannel (Variables|Default|GetCapsuleComponent) "ECC_WorldDynamic" "ECR_Ignore")
    (Collision|SetCollisionResponsetoChannel (Variables|Default|GetCapsuleComponent) "ECC_Pawn" "ECR_Ignore")
    (Utilities|FlowControl|Delay 3.0)
    (Actor|DestroyActor)))

(fn ConstructionScript
  (|CallParentFunction)
  ;[0.15 0.15 0.15 0.5] Set Mesh Color
  (bind _returnvalue (Rendering|Material|CreateDynamicMaterialInstance (Variables|Character|GetMesh) 0 0 "None" :!class /Script/Engine.PrimitiveComponent))
  (bind _output_get (Variables|Default|SetBodyMat _returnvalue))
  (Rendering|Material|SetVectorParameterValue _output_get "BodyColor" (Variables|Default|GetBodyColor) :!class /Script/Engine.MaterialInstanceDynamic))

(fn QuantizeMeshRotation
  (params (NewParam :type Rotator))
  (Transformation|SetWorldRotation (Variables|Character|GetMesh) (Math|Rotator|MakeRotator 0.0 0.0 (Math|Conversions|ToFloat(Integer) (- (* (Math|Float|Round (/ (.yaw NewParam) 45.0)) 45) 90))) false false))