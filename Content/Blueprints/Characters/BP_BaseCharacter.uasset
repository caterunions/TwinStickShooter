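; BP_BaseCharacter is a base character Blueprint that provides basic health tracking.
; BeginPlay fills Health from MaxHealth.
; CalculateHealth adds a signed delta and clamps the result between zero and MaxHealth.
; IsDead reports whether Health is at or below zero, but the event graph does not act on it.
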(event EventBeginPlay
  (Variables|BaseCharacter|SetHealth (Variables|BaseCharacter|GetMaxHealth)))

(fn ConstructionScript)

(fn IsDead
  (return (<= (Variables|BaseCharacter|GetHealth) 0.0)))

(fn CalculateHealth
  (params (Delta :type Float%20%28double-precision%29))
  (Variables|BaseCharacter|SetHealth (Math|Float|Min(Float) (Math|Float|Max(Float) (+ Delta (Variables|BaseCharacter|GetHealth)) 0.0) (Variables|BaseCharacter|GetMaxHealth)))
  (return))