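; BP_MeleeWeaponPickup is an interactable pickup that gives the player a melee weapon.
; It overrides AddWeapon, running the parent logic and then casting the WeaponMesh component's skinned asset to a SkeletalMesh.
; On a successful cast it adds a BP melee weapon component to the Player, passing that mesh plus the pickup's attack and damage stats.
; The event graph and construction script add no logic of their own.
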(event EventBeginPlay
  (|CallParentFunction) ; This node is disabled and will not be called.\nDrag off pins to build functionality.
)

(event Collision|EventActorBeginOverlap
  (params (OtherActor :type Actor%20Object%20Reference))
  (|CallParentFunction OtherActor) ; This node is disabled and will not be called.\nDrag off pins to build functionality.
)

(event EventTick
  (params (DeltaSeconds :type Float%20%28single-precision%29))
  (|CallParentFunction DeltaSeconds) ; This node is disabled and will not be called.\nDrag off pins to build functionality.
)

(fn ConstructionScript
  (|CallParentFunction))

(fn AddWeapon
  (|CallParentFunction)
  (bind _asskeletal_mesh (Utilities|Casting|CastToSkeletalMesh (Class|SkinnedMeshComponent|GetSkinnedAsset (Variables|Default|GetWeaponMesh))))
  (AddComponent|AddBPMeleeWeaponComponent :self (Variables|Default|GetPlayer) :AttackRange (Variables|Default|GetAttack%20Range) :AttackAngle (Variables|Default|GetAttack%20Angle) :BaseAttackTIme (Variables|Default|GetBase%20Attack%20TIme) :WeaponMesh _asskeletal_mesh :BaseDamage (Variables|Default|GetBase%20Damage)))