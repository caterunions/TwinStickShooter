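; BP_WeaponPickup is an interactable weapon pickup that swaps the player's current weapon for a new one.
; On interact, it searches the player mesh's direct child components for a BP_Weapon_Component, spawns that weapon's pickup class at the player's transform, and destroys the weapon.
; It then calls AddWeapon, left empty here as an apparent hook for child Blueprints, and destroys itself.
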(event EventBeginPlay
  (|CallParentFunction) ; This node is disabled and will not be called.\nDrag off pins to build functionality.
)

(event Collision|EventActorBeginOverlap
  (params (OtherActor :type Actor%20Object%20Reference)))

(event EventTick
  (params (DeltaSeconds :type Float%20%28single-precision%29)))

(fn ConstructionScript
  (|CallParentFunction))

(fn OnInteract
  (bind _player (Variables|Default|GetPlayer))
  (|CallParentFunction)
  (Variables|WeaponPickupBase|SetPlayerHasWeapon false)
  (bind _array_element (Utilities|Array|ForEachLoopwithBreak (Components|GetChildrenComponents (Variables|/Script/Engine.Character|GetMesh (Variables|Default|GetPlayer)) false) :!label _label)
    (:LoopBody
      (bind _asbp_weapon_component (Utilities|Casting|CastToBP_Weapon_Component _array_element))
      (Variables|Default|SetPreviousWeapon _asbp_weapon_component)
      (Variables|WeaponPickupBase|SetPlayerHasWeapon true)
      (goto _label Break))
    (:Completed
      (if (Variables|WeaponPickupBase|GetPlayerHasWeapon)
        (if (Utilities|IsValidClass (Variables|/Game/Blueprints/Weapons/BP_Weapon_Component.BP_Weapon_Component_C|GetPickup (Variables|Default|GetPreviousWeapon)))
          (Game|SpawnActorfromClass (Variables|/Game/Blueprints/Weapons/BP_Weapon_Component.BP_Weapon_Component_C|GetPickup (Variables|Default|GetPreviousWeapon)) (Transformation|GetActorTransform _player) "AlwaysSpawn" "MultiplyWithRoot" 0 0))
        (Default|DestroyWeapon _player (Variables|Default|GetPreviousWeapon)))
      (CallFunction|AddWeapon)
      (Actor|DestroyActor))))

(fn AddWeapon)