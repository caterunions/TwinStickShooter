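; BP_Interactable is an interactable actor with an empty OnInteract function, which randomly destroys itself on BeginPlay according to SpawnChance.
; Range overlap with BP_HeroCharacter and cursor hover over MouseHitbox jointly reveal an arrow, and losing either hides it.
; While shown, a looping timer runs UpdateArrowPos, bobbing the arrow by adding a time-based sine to its current Z.
; The saved ArrowStartZ is unused here, and the click event is empty.
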(event OnBeginCursorOver(MouseHitbox)
  (params (TouchedComponent :type Primitive%20Component%20Object%20Reference))
  ;[0.15 0.15 0.15 0.5] Cursor Begin Hover
  (Variables|Default|SetMouseOver true)
  (if (Variables|Default|GetPlayerInRange)
    ;[0.15 0.15 0.15 0.5] Show Arrow
    (Rendering|SetVisibility (Variables|Default|GetArrow) true false)
    (Utilities|Time|SetTimerbyFunctionName 0 "UpdateArrowPos" 0.01 true true)))

(event OnClicked(MouseHitbox)
  (params (TouchedComponent :type Primitive%20Component%20Object%20Reference) (ButtonPressed :type Key%20Structure :default "None")))

(event OnEndCursorOver(MouseHitbox)
  (params (TouchedComponent :type Primitive%20Component%20Object%20Reference))
  ;[0.15 0.15 0.15 0.5] Cursor End Hover
  (Variables|Default|SetMouseOver false)
  ;[0.15 0.15 0.15 0.5] Hide Arrow
  (Rendering|SetVisibility (Variables|Default|GetArrow) false false)
  (Utilities|Time|ClearTimerbyFunctionName 0 "UpdateArrowPos"))

(event OnComponentBeginOverlap(PlayerInteractionRange)
  (params (OverlappedComponent :type Primitive%20Component%20Object%20Reference) (OtherActor :type Actor%20Object%20Reference) (OtherComp :type Primitive%20Component%20Object%20Reference) (OtherBodyIndex :type Integer) (bFromSweep :type Boolean) (SweepResult :type Hit%20Result%20Structure%20%28by%20ref%29))
  ;[0.15 0.15 0.15 0.5] Player Overlap
  (bind _asbp_hero_character (Utilities|Casting|CastToBP_HeroCharacter OtherActor))
  (Variables|Default|SetPlayer _asbp_hero_character)
  (Variables|Default|SetPlayerInRange true)
  (if (Variables|Default|GetMouseOver)
    ;[0.15 0.15 0.15 0.5] Show Arrow
    (Rendering|SetVisibility (Variables|Default|GetArrow) true false)
    (Utilities|Time|SetTimerbyFunctionName 0 "UpdateArrowPos" 0.01 true true)))

(event OnComponentEndOverlap(PlayerInteractionRange)
  (params (OverlappedComponent :type Primitive%20Component%20Object%20Reference) (OtherActor :type Actor%20Object%20Reference) (OtherComp :type Primitive%20Component%20Object%20Reference) (OtherBodyIndex :type Integer))
  ;[0.15 0.15 0.15 0.5] Player End Overlap
  (Utilities|Casting|CastToBP_HeroCharacter OtherActor)
  (Variables|Default|SetPlayerInRange false)
  ;[0.15 0.15 0.15 0.5] Hide Arrow
  (Rendering|SetVisibility (Variables|Default|GetArrow) false false)
  (Utilities|Time|ClearTimerbyFunctionName 0 "UpdateArrowPos"))

(event EventBeginPlay
  ;[0.15 0.15 0.15 0.5] BeginPlay
  (Utilities|FlowControl|Sequence
    (:then_0
      ;;[0.15 0.15 0.15 0.5] Roll chance to not spawn
      (if (> (Math|Random|RandomFloat) (Variables|Default|GetSpawnChance))
        (Actor|DestroyActor)))
    (:then_1
      ;;[0.15 0.15 0.15 0.5] Hide Arrow and save Z position
      (Rendering|SetVisibility (Variables|Default|GetArrow) false false)
      (Variables|Default|SetArrowStartZ (.z (Transformation|GetWorldLocation (Variables|Default|GetArrow)))))))

(fn ConstructionScript)

(fn UpdateArrowPos
  (bind _arrow (Variables|Default|GetArrow))
  (bind _returnvalue (Transformation|GetWorldLocation _arrow))
  (Transformation|SetWorldLocation (Variables|Default|GetArrow) (Math|Vector|MakeVector (.x _returnvalue) (.y _returnvalue) (+ (.z _returnvalue) (Math|Trig|Sin(Radians) (* (Utilities|Time|GetTimeSeconds) 5.0)))) false false))

(fn OnInteract)