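; Weapon Blueprint that provides automatic projectile fire for the player.
; BeginFiring passes a DoOnce gate, fires immediately, then starts a looping timer that calls Fire at the ShotsPerSecond rate.
; Fire spawns BP_Projectile at the Player's ProjectileLauncher transform.
; EndFiring clears the timer and resets the gate, so the next BeginFiring shoots instantly with no cooldown.
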(event Custom|BeginFiring
  (params (NewParam :type Transform))
  (Utilities|FlowControl|DoOnce false
    (:Completed
      (CallFunction|Fire)
      (Utilities|Time|SetTimerbyFunctionName 0 "Fire" (/ 1.0 (Variables|Default|GetShotsPerSecond)) true))))

(event Custom|EndFiring
  (Utilities|Time|ClearTimerbyFunctionName 0 "Fire")
  (Utilities|FlowControl|DoOnce false) ; enters at Reset
)

(event Custom|Fire
  ;[0.15 0.15 0.15 0.5] Fire
  (Game|SpawnActorfromClass "/Game/Blueprints/BP_Projectile.BP_Projectile_C" (Transformation|GetWorldTransform (Variables|/Game/Blueprints/BP_HeroCharacter.BP_HeroCharacter_C|GetProjectileLauncher (Variables|Default|GetPlayer))) "Undefined" "MultiplyWithRoot" 0 0))

(fn ConstructionScript)