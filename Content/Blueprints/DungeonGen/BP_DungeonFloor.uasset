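; BP_DungeonFloor is a procedural dungeon floor actor that tiles a Length by Width grid with instanced mesh pieces.
; The Construction Script loops over the grid and adds an evenly spaced instance to a randomly chosen floor component per cell.
; Repeated entries in the pick array weight the result toward the first floor variant, and random quarter-turn yaw breaks up repetition.
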(event EventBeginPlay)

(event Collision|EventActorBeginOverlap
  (params (OtherActor :type Actor%20Object%20Reference)))

(event EventTick
  (params (DeltaSeconds :type Float%20%28single-precision%29)))

(fn ConstructionScript
  (for _index (range 0 (- (Variables|Default|GetLength) 1))
    (for _index_2 (range 0 (- (Variables|Default|GetWidth) 1))
      (Components|InstancedStaticMesh|AddInstance (.OutItem (Utilities|Array|Random (Utilities|Array|MakeArray (Variables|Default|GetFloorInstance1) (Variables|Default|GetFloorInstance2) (Variables|Default|GetFloorInstance3) (Variables|Default|GetFloorInstance4) (Variables|Default|GetFloorInstance5) (Variables|Default|GetFloorInstance6) (Variables|Default|GetFloorInstance7) (Variables|Default|GetFloorInstance1) (Variables|Default|GetFloorInstance1) (Variables|Default|GetFloorInstance1) (Variables|Default|GetFloorInstance1) (Variables|Default|GetFloorInstance1) (Variables|Default|GetFloorInstance1)))) (Math|Transform|MakeTransform (Math|Vector|MakeVector (Math|Conversions|ToFloat(Integer) (* _index 210)) (Math|Conversions|ToFloat(Integer) (* _index_2 210)) 0.0) (Math|Rotator|MakeRotator 0.0 0.0 (Math|Conversions|ToFloat(Integer) (* (Math|Random|RandomInteger 5) 90))) "1.000000,1.000000,1.000000") false))))