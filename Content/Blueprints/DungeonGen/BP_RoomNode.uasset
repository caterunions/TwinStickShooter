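; BP_RoomNode is a dungeon generation connection point that spawns a random room when the hero enters its sphere, or already overlaps it after BeginPlay.
; Once three or more nodes exist, dead ends join the random pool.
; Rooms spawn with a small forward offset and only if collision-free; otherwise a BP_DoorBlocker is placed instead.
; The node prints the result and destroys itself.
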(event OnComponentBeginOverlap(Sphere)
  (params (OverlappedComponent :type Primitive%20Component%20Object%20Reference) (OtherActor :type Actor%20Object%20Reference) (OtherComp :type Primitive%20Component%20Object%20Reference) (OtherBodyIndex :type Integer) (bFromSweep :type Boolean) (SweepResult :type Hit%20Result%20Structure%20%28by%20ref%29))
  (bind _sphere (Variables|Default|GetSphere))
  (bind _returnvalue (Transformation|GetWorldTransform _sphere))
  (bind _returnvalue_2 (Math|Vector|GetForwardVector _sphere))
  (bind _returnvalue_3 (+ _returnvalue_2 (.location _returnvalue)))
  (bind _returnvalue_4 (Math|Transform|MakeTransform _returnvalue_3 (.rotation _returnvalue) (.scale _returnvalue)))
  ;[0.15 0.15 0.15 0.5] Check Character Overlap
  (Utilities|Casting|CastToBP_HeroCharacter OtherActor)
  ;[0.15 0.15 0.15 0.5] If 3 or more room nodes existing
  (bind _outactors (Actor|GetAllActorsOfClass "BP_RoomNode_C"))
  (if (>= (Utilities|Array|Length _outactors) 3)
    (Utilities|Array|AppendArray (Variables|Default|GetRooms) (Variables|Default|GetDead%20Ends)))
  ;[0.15 0.15 0.15 0.5] Spawn Random Room
  (bind _returnvalue_5 (Game|SpawnActorfromClass (.OutItem (Utilities|Array|Random (Variables|Default|GetRooms))) _returnvalue_4 "DontSpawnIfColliding" "MultiplyWithRoot" 0 0))
  (if (Utilities|IsValid _returnvalue_5)
    ;[0.15 0.15 0.15 0.5] Room Spawned Successfully
    (Development|PrintString (Utilities|String|ToString(Text) (Utilities|Text|FormatText "Room '{Room}' Created" (Utilities|GetDisplayName _returnvalue_5))))
    (else
      ;[0.15 0.15 0.15 0.5] Room Failed to Spawn
      (Development|PrintString "Room Failed To Spawn")
      (Game|SpawnActorfromClass "/Game/Blueprints/DungeonGen/BP_DoorBlocker.BP_DoorBlocker_C" _returnvalue_4 "AlwaysSpawn" "MultiplyWithRoot" 0 0)))
  ;[0.15 0.15 0.15 0.5] Destroy Room Node
  (Actor|DestroyActor))

(event EventBeginPlay
  (bind _sphere (Variables|Default|GetSphere))
  (bind _returnvalue (Transformation|GetWorldTransform _sphere))
  (bind _returnvalue_2 (Math|Vector|GetForwardVector _sphere))
  (bind _returnvalue_3 (+ _returnvalue_2 (.location _returnvalue)))
  (bind _returnvalue_4 (Math|Transform|MakeTransform _returnvalue_3 (.rotation _returnvalue) (.scale _returnvalue)))
  ;[0.15 0.15 0.15 0.5] Check if player is within node spawn radius when it is created
  (Utilities|FlowControl|DelayUntilNextTick)
  (if (> (Utilities|Array|Length (Collision|GetOverlappingActors (Variables|Default|GetSphere) "/Game/Blueprints/Characters/BP_HeroCharacter.BP_HeroCharacter_C" :!class /Script/Engine.PrimitiveComponent)) 0)
    ;[0.15 0.15 0.15 0.5] If 3 or more room nodes existing
    (bind _outactors (Actor|GetAllActorsOfClass "BP_RoomNode_C"))
    (if (>= (Utilities|Array|Length _outactors) 3)
      (Utilities|Array|AppendArray (Variables|Default|GetRooms) (Variables|Default|GetDead%20Ends)))
    ;[0.15 0.15 0.15 0.5] Spawn Random Room
    (bind _returnvalue_5 (Game|SpawnActorfromClass (.OutItem (Utilities|Array|Random (Variables|Default|GetRooms))) _returnvalue_4 "DontSpawnIfColliding" "MultiplyWithRoot" 0 0))
    (if (Utilities|IsValid _returnvalue_5)
      ;[0.15 0.15 0.15 0.5] Room Spawned Successfully
      (Development|PrintString (Utilities|String|ToString(Text) (Utilities|Text|FormatText "Room '{Room}' Created" (Utilities|GetDisplayName _returnvalue_5))))
      (else
        ;[0.15 0.15 0.15 0.5] Room Failed to Spawn
        (Development|PrintString "Room Failed To Spawn")
        (Game|SpawnActorfromClass "/Game/Blueprints/DungeonGen/BP_DoorBlocker.BP_DoorBlocker_C" _returnvalue_4 "AlwaysSpawn" "MultiplyWithRoot" 0 0)))
    ;[0.15 0.15 0.15 0.5] Destroy Room Node
    (Actor|DestroyActor)))

(fn ConstructionScript)