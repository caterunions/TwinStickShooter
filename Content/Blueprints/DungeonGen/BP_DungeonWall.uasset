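; BP_DungeonWall is a dungeon wall actor that builds a straight run of wall segments from its Length value.
; The construction script loops over the segment count, adding each instance at an even spacing along local X.
; Each segment picks randomly among six instanced mesh components, weighted toward WallInstance0 by repeating it in the selection array.
; The event graph holds no active logic.
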(event EventBeginPlay)

(event Collision|EventActorBeginOverlap
  (params (OtherActor :type Actor%20Object%20Reference)))

(event EventTick
  (params (DeltaSeconds :type Float%20%28single-precision%29)))

(fn ConstructionScript
  (for _index (range 0 (- (Variables|Default|GetLength) 1))
    (Components|InstancedStaticMesh|AddInstance (.OutItem (Utilities|Array|Random (Utilities|Array|MakeArray (Variables|Default|GetWallInstance0) (Variables|Default|GetWallInstance1) (Variables|Default|GetWallInstance2) (Variables|Default|GetWallInstance3) (Variables|Default|GetWallInstance4) (Variables|Default|GetWallInstance5) (Variables|Default|GetWallInstance0) (Variables|Default|GetWallInstance0) (Variables|Default|GetWallInstance0) (Variables|Default|GetWallInstance0) (Variables|Default|GetWallInstance0)))) (Math|Transform|MakeTransform (Math|Vector|MakeVector (Math|Conversions|ToFloat(Integer) (* _index 210)) 0.0 0.0) "0, 0, 0" "1.000000,1.000000,1.000000") false)))