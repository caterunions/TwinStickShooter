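; Enemy character that takes damage through IDamageable, destroys itself when dead, and hurts the hero on contact.
; Overlapping the DamageVolume caches the hero and starts a looping timer that applies Damage until that hero leaves the volume.
; Each tick snaps the mesh yaw to eight-way 45-degree steps from the capsule rotation, with a -90 offset.
; The construction script tints the mesh with BodyColor through a dynamic material.
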(event OnComponentBeginOverlap(DamageVolume)
  (params (OverlappedComponent :type Primitive%20Component%20Object%20Reference) (OtherActor :type Actor%20Object%20Reference) (OtherComp :type Primitive%20Component%20Object%20Reference) (OtherBodyIndex :type Integer) (bFromSweep :type Boolean) (SweepResult :type Hit%20Result%20Structure%20%28by%20ref%29))
  (bind _asbp_hero_character (Utilities|Casting|CastToBP_HeroCharacter OtherActor))
  (Variables|Default|SetHero _asbp_hero_character)
  (Utilities|Time|SetTimerbyFunctionName 0 "DamageHero" 0.5 true))

(event OnComponentEndOverlap(DamageVolume)
  (params (OverlappedComponent :type Primitive%20Component%20Object%20Reference) (OtherActor :type Actor%20Object%20Reference) (OtherComp :type Primitive%20Component%20Object%20Reference) (OtherBodyIndex :type Integer))
  (if (== OtherActor (Variables|Default|GetHero))
    (Utilities|Time|ClearTimerbyFunctionName 0 "DamageHero")))

(event Custom|DamageHero
  (Default|AffectHealth (Variables|Default|GetHero) (* (Variables|Default|GetDamage) -1.0)))

(event EventTick
  (params (DeltaSeconds :type Float%20%28single-precision%29))
  (CallFunction|QuantizeMeshRotation (Transformation|GetWorldRotation (Variables|Default|GetCapsuleComponent))))

(event EventAffectHealth
  (params (Delta :type Float%20%28double-precision%29))
  ;[0.15 0.15 0.15 0.5] Implement IDamageable
  (CallFunction|CalculateHealth Delta)
  (if (CallFunction|IsDead)
    (Actor|DestroyActor)))

(fn ConstructionScript
  (|CallParentFunction)
  ;[0.15 0.15 0.15 0.5] Set Mesh Color
  (bind _returnvalue (Rendering|Material|CreateDynamicMaterialInstance (Variables|Character|GetMesh) 0 0 "None" :!class /Script/Engine.PrimitiveComponent))
  (bind _output_get (Variables|Default|SetBodyMat _returnvalue))
  (Rendering|Material|SetVectorParameterValue _output_get "BodyColor" (Variables|Default|GetBodyColor) :!class /Script/Engine.MaterialInstanceDynamic))

(fn QuantizeMeshRotation
  (params (NewParam :type Rotator))
  (Transformation|SetWorldRotation (Variables|Character|GetMesh) (Math|Rotator|MakeRotator 0.0 0.0 (Math|Conversions|ToFloat(Integer) (- (* (Math|Float|Round (/ (.yaw NewParam) 45.0)) 45) 90))) false false))